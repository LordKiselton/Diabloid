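; BP_RipSaw is a saw trap whose RotorBlade slides along a track while spinning.
; On BeginPlay, Timeline_0 starts after a random delay of up to three seconds and lerps the blade's relative location along local Y, so instances can fall out of sync.
; The Rotor timeline drives the blade's roll in parallel, starting without waiting for that delay.
; The graph contains no active overlap or damage logic.
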(event EventBeginPlay
  (bind _rotorblade (Variables|Default|GetRotorBlade))
  (Utilities|FlowControl|Sequence
    (:then_0
      (Utilities|FlowControl|Delay (Math|Float|Lerp 3.0 0.0 (Math|Random|RandomFloat)))
      (bind _move (Timeline|Timeline_0 Play)
        (:Update
          (Transformation|SetRelativeLocation _rotorblade (Math|Vector|Lerp(Vector) "0.000000,0.000000,4.570000" "0.000000,220.000000,4.570000" _move) false false))))
    (:then_1
      (bind _newtrack_0 (Timeline|Rotor Play)
        (:Update
          (Transformation|SetRelativeRotation _rotorblade (Math|Rotator|MakeRotator _newtrack_0 0.0 0.0) false false))))))

(event Collision|EventActorBeginOverlap
  (params (OtherActor :type Actor%20Object%20Reference)))

(event EventTick
  (params (DeltaSeconds :type Float%20%28single-precision%29)))

(fn ConstructionScript)